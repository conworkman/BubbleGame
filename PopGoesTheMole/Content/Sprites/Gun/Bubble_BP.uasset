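; Bubble actor, filed with the gun sprites, that slows to a stop and pops after a fixed lifetime.
; While moving, Tick brakes the Box's physics velocity by SlowDownFactor, choosing the sign from Y velocity, until speed nears zero.
; Overlapping another Bubble_BP shows that bubble's pop animation, then destroys both after a brief delay.
; Popping swaps the front and back bubble visuals for PopAnim by toggling visibility.
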(event `self.ReceiveTick`
  (params (DeltaSeconds :type "Float (single-precision)"))
  (bind _box (`self.Box`))
  (bind _box_2 (`self.Box`))
  (bind _returnvalue (`SceneComponent.GetComponentVelocity` _box))
  (bind _returnvalue_2 (`SceneComponent.GetComponentVelocity` _box_2))
  (if (`self.Moving`)
    (if (> (.y _returnvalue_2) 0.0)
      (`PrimitiveComponent.SetPhysicsLinearVelocity` _box_2 (- _returnvalue_2 (* (`self.SlowDownFactor`) DeltaSeconds)) false "None")
      (if (`KismetMathLibrary.NearlyEqual_FloatFloat` (`KismetMathLibrary.VSize` _returnvalue_2) 0.0 1.0)
        (set `self.Moving` false))
      (else
        (`PrimitiveComponent.SetPhysicsLinearVelocity` _box (+ _returnvalue (* (`self.SlowDownFactor`) DeltaSeconds)) false "None")
        (if (`KismetMathLibrary.NearlyEqual_FloatFloat` (`KismetMathLibrary.VSize` _returnvalue) 0.0 1.0)
          (set `self.Moving` false))))))

(event `self.ReceiveActorBeginOverlap`
  (params (OtherActor :type "Actor Object Reference"))
  (bind _asbubble_bp (cast `/Game/Sprites/Gun/Bubble_BP` OtherActor))
  (`self.PopAnimation` _asbubble_bp)
  (`KismetSystemLibrary.Delay` 0.025)
  (`self.DestroyBubbleSmall` _asbubble_bp)
  (`self.DestroyBubbleSmall`))

(event `self.ReceiveBeginPlay`
  (`KismetSystemLibrary.Delay` 7.5)
  (`self.PopAnimation`)
  (`KismetSystemLibrary.Delay` 0.025)
  (`self.DestroyBubbleSmall`))

(fn `DestroyBubbleSmall`
  (`self.K2_DestroyActor`))

(fn `PopAnimation`
  (`SceneComponent.SetVisibility` (`self.BubbleAnimationBack`) false false)
  (`SceneComponent.SetVisibility` (`self.BubbleAnimationFront`) false false)
  (`SceneComponent.SetVisibility` (`self.PopAnim`) true false))

(fn `UserConstructionScript`)